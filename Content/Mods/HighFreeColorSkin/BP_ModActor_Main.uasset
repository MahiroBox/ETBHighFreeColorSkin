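; Mod actor for HighFreeColorSkin that toggles the mod's WBP_Main menu with the N key, only when the local pawn has authority.
; It polls the key on Tick, creating the widget if none is valid after removing stale copies, otherwise flipping its visibility.
; Opening sets Game and UI input with a cursor; closing restores game-only input and hides the cursor, except on MainMenuMap.
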(event EventTick
  (params (DeltaSeconds :type Float%20%28single-precision%29))
  (bind _returnvalue (Game|GetPlayerController 0))
  (bind _returnvalue_2 (Game|GetPlayerController 0))
  (if (Game|Player|WasInputKeyJustPressed (Game|GetPlayerController 0) "N")
    (if (Ability|HasAuthority (Game|Player|GetPlayerPawn 0))
      (Utilities|IsValid (Variables|Default|GetMenu)
        (:Is%20Valid
          (switch Utilities|FlowControl|Switch|SwitchonESlateVisibility (Widget|GetVisibility (Variables|Default|GetMenu))
            (:Visible
              (Widget|SetVisibility (Variables|Default|GetMenu) "Collapsed" :!label _label)
              (bind _returnvalue_3 (Game|GetCurrentLevelName true))
              (if (Utilities|Enum|NotEqual(Enum) _returnvalue_3 "MainMenuMap")
                (Input|SetInputModeGameOnly _returnvalue)
                (Variables|/Script/Engine.PlayerController|SetbShowMouseCursor _returnvalue false)))
            (:Collapsed
              (Widget|SetVisibility (Variables|Default|GetMenu) "SelfHitTestInvisible" :!label _label_2)
              (Input|SetInputModeGameandUI (Game|GetPlayerController 0) (Variables|Default|GetMenu) "DoNotLock" true :!label _label_3)
              (Variables|/Script/Engine.PlayerController|SetbShowMouseCursor _returnvalue_2 true))
            (:Hidden
              (goto _label_2))
            (:HitTestInvisible
              (goto _label))
            (:SelfHitTestInvisible
              (goto _label))))
        (:Is%20Not%20Valid
          (bind _foundwidgets (Widget|GetAllWidgetsOfClass "/Game/Mods/HighFreeColorSkin/WBP_Main.WBP_Main_C" true))
          (Widget|RemovefromParent _foundwidgets)
          (bind _returnvalue_4 (UserInterface|CreateWidget "/Game/Mods/HighFreeColorSkin/WBP_Main.WBP_Main_C" _returnvalue_2))
          (bind _output_get (Variables|Default|SetMenu _returnvalue_4))
          (UserInterface|Viewport|AddtoViewport _output_get 1)
          (Widget|SetVisibility _output_get "Visible")
          (goto _label_3))))))

(fn ConstructionScript)